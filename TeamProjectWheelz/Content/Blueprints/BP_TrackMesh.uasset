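; BP_TrackMesh is a track actor that lays a chosen mesh repeatedly along a spline.
; Its construction script steps by the mesh's X extent, adding spline mesh components with configurable collision, size-clamped tangents and a MeshBuffer offset on each end position.
; It also recolors the spline's editor display.
; On BeginPlay, if RandoizeColor is set, it randomizes every vector parameter in the material parameter collection.
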(event `self.ReceiveBeginPlay`
  (bind _materialparametercollection (`self.MaterialParameterCollection`))
  (if (`self.RandoizeColor`)
    (for _array_element (`MaterialParameterCollection.GetVectorParameterNames` _materialparametercollection)
      (`KismetMaterialLibrary.SetVectorParameterValue` _materialparametercollection _array_element (`KismetMathLibrary.MakeColor` (`KismetMathLibrary.RandomFloatInRange` 0.0 1.0) (`KismetMathLibrary.RandomFloatInRange` 0.0 1.0) (`KismetMathLibrary.RandomFloatInRange` 0.0 1.0))))))

(event `self.ReceiveActorBeginOverlap`
  (params (OtherActor :type "Actor Object Reference")))

(fn `UserConstructionScript`
  (bind _spline (`self.Spline`))
  (bind _spline_2 (`self.Spline`))
  (bind _xlength (`self.XLength`))
  (bind _spline_3 (`self.Spline`))
  (bind (_returnvalue_min _returnvalue_max) (break `Box` (`StaticMesh.GetBoundingBox` (`self.Mesh`))))
  (bind _returnvalue_x (`KismetMathLibrary.BreakVector` (+ (`KismetMathLibrary.Vector_GetAbs` _returnvalue_min) (`KismetMathLibrary.Vector_GetAbs` _returnvalue_max))))
  (set `self.XLength` _returnvalue_x)
  (for _index (range (+ (`KismetMathLibrary.FTrunc` (/ (`SplineComponent.GetSplineLength` (`self.Spline`)) (`self.XLength`))) 1))
    (bind _returnvalue (`AddComponent|NODE_AddSplineMeshComponent-0`))
    (`PrimitiveComponent.SetCollisionEnabled` _returnvalue (`self.Collision Type`))
    (`SplineMeshComponent.SetForwardAxis` _returnvalue "X" true)
    (`StaticMeshComponent.SetStaticMesh` _returnvalue (`self.Mesh`))
    (bind _returnvalue_2 (* _index (`self.XLength`)))
    (bind _returnvalue_3 (* (+ _index 1.0) (`self.XLength`)))
    (`SplineMeshComponent.SetStartAndEnd` _returnvalue (`SplineComponent.GetLocationAtDistanceAlongSpline` _spline_2 _returnvalue_2 "Local") (`KismetMathLibrary.ClampVectorSize` (`SplineComponent.GetTangentAtDistanceAlongSpline` _spline_2 _returnvalue_2 "Local") 0.0 _xlength) (`SplineComponent.GetLocationAtDistanceAlongSpline` _spline_3 (- _returnvalue_3 (`self.Mesh Buffer`)) "Local") (`KismetMathLibrary.ClampVectorSize` (`SplineComponent.GetTangentAtDistanceAlongSpline` _spline_3 _returnvalue_3 "Local") _xlength) true)
    (`SplineComponent.SetUnselectedSplineSegmentColor` _spline (make `LinearColor` 1.0 0.0 1.0 1.0))
    (`SplineComponent.SetSelectedSplineSegmentColor` _spline (make `LinearColor` 1.0 1.0 0.0 1.0))
    (`SplineComponent.SetTangentColor` _spline (make `LinearColor` 0.0 1.0 1.0 1.0))))