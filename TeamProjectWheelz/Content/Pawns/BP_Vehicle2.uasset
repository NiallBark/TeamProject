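; Drivable vehicle pawn with a pre-drive door customizer and mouse-driven camera rotation.
; Before the game starts, right-clicking either door box line-traces from the cursor and steps both doors through three clamped mesh options.
; The TestMapping action enables driving input and unlocks the spring arm from control rotation.
; V saves the door meshes and vehicle class, then opens BaseLevel; BeginPlay restores the saved meshes.
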(event `self.ReceiveBeginPlay`
  ;[1 1 1] BeginPlay
  (set `PlayerController.bShowMouseCursor` true (`GameplayStatics.GetPlayerController` 0))
  (set `self.IsGameStarted` false)
  (if (`KismetSystemLibrary.IsValid` "/Game/Blueprints/BP_SaveGameState.BP_SaveGameState")
    (bind _returnvalue (`GameplayStatics.LoadGameFromSlot` "1"))
    (bind _asbp_save_game_state (cast `/Game/Blueprints/BP_SaveGameState` _returnvalue))
    (`StaticMeshComponent.SetStaticMesh` (`self.Door`) (`/Game/Blueprints/BP_SaveGameState.MeshObjRef1` _asbp_save_game_state))
    (`StaticMeshComponent.SetStaticMesh` (`self.Door2`) (`/Game/Blueprints/BP_SaveGameState.MeshObjRef2` _asbp_save_game_state))))

(event `InputAction|TestMapping`
  (params (Key :type "Key Structure"))
  ;[1 1 1] TESTUBG
  (:`Pressed`
    (set `self.IsGameStarted` true)
    (set `SpringArmComponent.bUsePawnControlRotation` false (`self.SpringArm`))))

(event `InputAxis|Throttle`
  (params (AxisValue :type "Float (single-precision)"))
  ;[1 1 1] Driving Controls
  (if (`self.IsGameStarted`)
    (`ChaosVehicleMovementComponent.SetThrottleInput` (`self.VehicleMovementComponent`) AxisValue)
    (`KismetSystemLibrary.PrintText` "Hello")))

(event `Key|V`
  (params (Key :type "Key Structure"))
  ;[1 1 1] TESTUBG
  (:`Pressed`
    (bind _returnvalue (`GameplayStatics.CreateSaveGameObject` "/Game/Blueprints/BP_SaveGameState.BP_SaveGameState_C"))
    (set `/Game/Blueprints/BP_SaveGameState.MeshObjRef1` (`StaticMeshComponent.StaticMesh` (`self.Door`)) _returnvalue)
    (set `/Game/Blueprints/BP_SaveGameState.MeshObjRef2` (`StaticMeshComponent.StaticMesh` (`self.Door2`)) _returnvalue)
    (set `/Game/Blueprints/BP_SaveGameState.SelectedActor` "BP_Vehicle2_C" _returnvalue)
    (`GameplayStatics.SaveGameToSlot` _returnvalue "1")
    (`GameplayStatics.OpenLevel` "BaseLevel")))

(event `InputAxis|MoveRight`
  (params (AxisValue :type "Float (single-precision)"))
  ;[1 1 1] Driving Controls
  (if (`self.IsGameStarted`)
    (`ChaosVehicleMovementComponent.SetSteeringInput` (`self.VehicleMovementComponent`) AxisValue)))

(event `InputAxis|Brake`
  (params (AxisValue :type "Float (single-precision)"))
  ;[1 1 1] Driving Controls
  (if (`self.IsGameStarted`)
    (`ChaosVehicleMovementComponent.SetBrakeInput` (`self.VehicleMovementComponent`) AxisValue)))

(event `InputAxisKey|MouseX`
  (params (AxisValue :type "Float (single-precision)"))
  (bind (_returnvalue_roll _returnvalue_pitch _returnvalue_yaw) (`KismetMathLibrary.BreakRotator` (`self.GetControlRotation`)))
  ;[1 1 1] Camera Controls
  (`self.AddControllerYawInput` AxisValue)
  (`Controller.SetControlRotation` (`GameplayStatics.GetPlayerController` 0) (`KismetMathLibrary.MakeRotator` 0.0 _returnvalue_pitch _returnvalue_yaw)))

(event `InputAxisKey|MouseY`
  (params (AxisValue :type "Float (single-precision)"))
  ;[1 1 1] Camera Controls
  (`self.AddControllerPitchInput` AxisValue))

(event `Key|RightMouseButton`
  (params (Key :type "Key Structure"))
  (bind (_worldlocation _worlddirection) (`PlayerController.DeprojectMousePositionToWorld` (`GameplayStatics.GetPlayerController` 0)))
  ;[1 1 1] MeshSelection Line trace to box
  (:`Pressed`
    (if (not (`self.IsGameStarted`))
      (bind _outhit (`KismetSystemLibrary.LineTraceSingle` :`Start` _worldlocation :`End` (+ _worldlocation (* _worlddirection 10000.0)) :`TraceChannel` "TraceTypeQuery1" :`DrawDebugType` "Persistent" :`bIgnoreSelf` false))
      (if (== (`.HitComponent` (`GameplayStatics.BreakHitResult` _outhit)) (`self.Door2Box`))
        ;;[1 1 1] Increment Door Meshes Down
        (bind _output_get (set `self.DoorInt` (`KismetMathLibrary.Clamp` (- (`self.DoorInt`) 1) 0 2)))
        (switch `int` _output_get
          (:`0`
            (`StaticMeshComponent.SetStaticMesh` (`self.Door`) "/Game/TestStaticMesh/TubeInvis.TubeInvis")
            (`StaticMeshComponent.SetStaticMesh` (`self.Door2`) "/Game/TestStaticMesh/TubeInvis.TubeInvis"))
          (:`1`
            (`StaticMeshComponent.SetStaticMesh` (`self.Door`) "/Game/TestStaticMesh/Tube.Tube")
            (`StaticMeshComponent.SetStaticMesh` (`self.Door2`) "/Game/TestStaticMesh/Tube.Tube"))
          (:`2`
            (`StaticMeshComponent.SetStaticMesh` (`self.Door`) "/Game/TestStaticMesh/TubeShadow.TubeShadow")
            (`StaticMeshComponent.SetStaticMesh` (`self.Door2`) "/Game/TestStaticMesh/TubeShadow.TubeShadow")))
        (elif (== (`.HitComponent` (`GameplayStatics.BreakHitResult` _outhit)) (`self.DoorBox`))
          ;;[1 1 1] Increment Door Meshes up
          (bind _output_get_2 (set `self.DoorInt` (`KismetMathLibrary.Clamp` (+ (`self.DoorInt`) 1) 0 2)))
          (switch `int` _output_get_2
            (:`0`
              (`StaticMeshComponent.SetStaticMesh` (`self.Door`) "/Game/TestStaticMesh/TubeInvis.TubeInvis")
              (`StaticMeshComponent.SetStaticMesh` (`self.Door2`) "/Game/TestStaticMesh/TubeInvis.TubeInvis"))
            (:`1`
              (`StaticMeshComponent.SetStaticMesh` (`self.Door`) "/Game/TestStaticMesh/Tube.Tube")
              (`StaticMeshComponent.SetStaticMesh` (`self.Door2`) "/Game/TestStaticMesh/Tube.Tube"))
            (:`2`
              (`StaticMeshComponent.SetStaticMesh` (`self.Door`) "/Game/TestStaticMesh/TubeShadow.TubeShadow")
              (`StaticMeshComponent.SetStaticMesh` (`self.Door2`) "/Game/TestStaticMesh/TubeShadow.TubeShadow"))))))))

(fn `UserConstructionScript`)