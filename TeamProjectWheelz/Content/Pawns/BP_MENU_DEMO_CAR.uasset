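; Customisable Chaos vehicle pawn that serves as both menu demo car and drivable car, with player or AI paint.
; BeginPlay applies saved parts and colour through dynamic materials, while customisation events change meshes and paint, saving to slot "1".
; Level name gates driving input, reset and teleport-to-start restart.
; It also handles mouse look, headlight toggling, rear-wheel friction drift updated on Tick, and a K-key skeletal mesh swap.
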(event `Key|K`
  (params (Key :type "Key Structure"))
  (bind _mesh (`self.Mesh`))
  (bind _mesh_2 (`self.Mesh`))
  (:`Pressed`
    (cast `/Game/Pawns/BP_BaseChaosCar` (`GameplayStatics.GetPlayerPawn` 0))
    (`SkeletalMeshComponent.SetSkeletalMeshAsset` _mesh_2 "/Game/Car2/tEST2/TestCar2.TestCar2")
    (`SkeletalMeshComponent.SetAnimInstanceClass` _mesh_2 "/Game/Car2/tEST2/ABP_Test2.ABP_Test2_C"))
  (:`Released`
    (`SkeletalMeshComponent.SetSkeletalMeshAsset` _mesh "/Game/RealCar1/lambo3.lambo3")
    (`SkeletalMeshComponent.SetAnimInstanceClass` _mesh "/Game/RealCar1/ABP_Lambo.ABP_Lambo_C")))

(event `self.ReceiveBeginPlay`
  (bind _mesh (`self.Mesh`))
  ;[1 1 1] BeginPlay
  (bind _returnvalue (`GameplayStatics.CreateSaveGameObject` "/Game/Blueprints/BP_SaveGameState.BP_SaveGameState_C"))
  (set `self.SaveGameState` _returnvalue)
  (set `PlayerController.bShowMouseCursor` true (`GameplayStatics.GetPlayerController` 0))
  (set `self.IsGameStarted` false)
  (if (`KismetSystemLibrary.IsValid` (`self.SaveGameState`))
    (bind _returnvalue_2 (`GameplayStatics.LoadGameFromSlot` "1"))
    (bind _asbp_save_game_state (cast `/Game/Blueprints/BP_SaveGameState` _returnvalue_2))
    (`self.SaveMeshConfig`)
    (`StaticMeshComponent.SetStaticMesh` (`self.Door`) (`/Game/Blueprints/BP_SaveGameState.DoorRef1` _asbp_save_game_state))
    (`StaticMeshComponent.SetStaticMesh` (`self.Door2`) (`/Game/Blueprints/BP_SaveGameState.DoorRef2` _asbp_save_game_state))
    (`StaticMeshComponent.SetStaticMesh` (`self.SM_Spoiler3`) (`/Game/Blueprints/BP_SaveGameState.SpoilerRef` _asbp_save_game_state))
    (`StaticMeshComponent.SetStaticMesh` (`self.SM_Bonnet`) (`/Game/Blueprints/BP_SaveGameState.BonnetRef` _asbp_save_game_state))
    (`self.StartDriving`)
    (`KismetSystemLibrary.Delay` 0.1)
    ;[1 1 1] Colour changer
    (if (`self.IsAI`)
      (bind _returnvalue_3 (`KismetMaterialLibrary.CreateDynamicMaterialInstance` "/Game/Materials/MTL_Base.MTL_Base"))
      (bind _returnvalue_4 (`KismetMaterialLibrary.CreateDynamicMaterialInstance` "/Game/Materials/MTL_SecondaryColour.MTL_SecondaryColour"))
      (`KismetSystemLibrary.Delay` 0.1)
      (`PrimitiveComponent.SetMaterial` _mesh 0 _returnvalue_3)
      (`MaterialInstanceDynamic.SetVectorParameterValue` _returnvalue_3 "BaseColour" (`self.AIColour`))
      (`PrimitiveComponent.SetMaterial` (`self.Mesh`) 1 _returnvalue_4)
      (`MaterialInstanceDynamic.SetVectorParameterValue` _returnvalue_3 "SecondaryColour" (`self.AISecondaryColour`))
      (`MaterialInstanceDynamic.SetVectorParameterValue` _returnvalue_4 "SecondaryColour" (`self.AISecondaryColour`))
      (else
        (bind _returnvalue_5 (`KismetMaterialLibrary.CreateDynamicMaterialInstance` "/Game/Materials/MTL_Base.MTL_Base"))
        (`KismetSystemLibrary.Delay` 0.1)
        (`PrimitiveComponent.SetMaterial` _mesh 0 _returnvalue_5)
        (bind _linearcoloursave (`/Game/Blueprints/BP_SaveGameState.LinearColourSave` _asbp_save_game_state))
        (`MaterialInstanceDynamic.SetVectorParameterValue` _returnvalue_5 "BaseColour" _linearcoloursave)
        (set `self.ParticleColor` _linearcoloursave)
        (`KismetSystemLibrary.PrintString` "loaded")))))

(event `StartDriving`
  ;[1 1 1] TESTUBG
  (bind _returnvalue (`GameplayStatics.GetCurrentLevelName` true))
  (if (or (`KismetStringLibrary.EqualEqual_StrStr` _returnvalue "Map2") (`KismetStringLibrary.EqualEqual_StrStr` _returnvalue "Map1") (`KismetStringLibrary.EqualEqual_StrStr` _returnvalue "BaseLevel"))
    (set `self.IsGameStarted` true)
    (set `SpringArmComponent.bUsePawnControlRotation` false (`self.CarSpringArm`))))

(event `ChangeColours`
  (params (LinearColour :type "LinearColor Structure"))
  ;[1 1 1] Colour changer
  (`MaterialInstanceDynamic.SetVectorParameterValue` (stale `self.ReceiveBeginPlay` _returnvalue_5) "BaseColour" LinearColour)
  (bind _output_get (set `/Game/Blueprints/BP_SaveGameState.LinearColourSave` LinearColour (`self.SaveGameState`)))
  (set `self.ParticleColor` _output_get)
  (`GameplayStatics.SaveGameToSlot` (`self.SaveGameState`) "1"))

(event `ChangeHue`
  (params (HueScalar :type "LinearColor Structure"))
  ;[1 1 1] Colour changer
  (`MaterialInstanceDynamic.SetVectorParameterValue` (stale `self.ReceiveBeginPlay` _returnvalue_5) "Hue" HueScalar))

(event `InputAxis|Throttle`
  (params (AxisValue :type "Float (single-precision)"))
  ;[1 1 1] Driving Controls
  (if (`self.IsGameStarted`)
    (`ChaosVehicleMovementComponent.SetThrottleInput` (`self.VehicleMovementComponent`) AxisValue)))

(event `SaveMeshConfig`
  (bind _savegamestate (`self.SaveGameState`))
  ;[1 1 1] TESTUBG
  (set `/Game/Blueprints/BP_SaveGameState.DoorRef1` (`StaticMeshComponent.StaticMesh` (`self.Door`)) _savegamestate)
  (set `/Game/Blueprints/BP_SaveGameState.DoorRef2` (`StaticMeshComponent.StaticMesh` (`self.Door2`)) _savegamestate)
  (set `/Game/Blueprints/BP_SaveGameState.SpoilerRef` (`StaticMeshComponent.StaticMesh` (`self.SM_Spoiler3`)) _savegamestate)
  (set `/Game/Blueprints/BP_SaveGameState.BonnetRef` (`StaticMeshComponent.StaticMesh` (`self.SM_Bonnet`)) _savegamestate)
  (set `/Game/Blueprints/BP_SaveGameState.SelectedActor` (`GameplayStatics.GetObjectClass` self) _savegamestate)
  (`GameplayStatics.SaveGameToSlot` _savegamestate "1"))

(event `ChangeMetallic`
  (params (Metallic :type "Float (double-precision)"))
  ;[1 1 1] Colour changer
  (`MaterialInstanceDynamic.SetScalarParameterValue` (stale `self.ReceiveBeginPlay` _returnvalue_5) "Metallic" Metallic))

(event `InputAxis|MoveRight`
  (params (AxisValue :type "Float (single-precision)"))
  ;[1 1 1] Driving Controls
  (if (`self.IsGameStarted`)
    (`ChaosVehicleMovementComponent.SetSteeringInput` (`self.VehicleMovementComponent`) AxisValue)))

(event `InputAxis|Brake`
  (params (AxisValue :type "Float (single-precision)"))
  ;[1 1 1] Driving Controls
  (if (`self.IsGameStarted`)
    (`ChaosVehicleMovementComponent.SetBrakeInput` (`self.VehicleMovementComponent`) AxisValue)))

(event `InputAxisKey|MouseX`
  (params (AxisValue :type "Float (single-precision)"))
  (bind (_returnvalue_roll _returnvalue_pitch _returnvalue_yaw) (`KismetMathLibrary.BreakRotator` (`self.GetControlRotation`)))
  ;[1 1 1] Camera Controls
  (`self.AddControllerYawInput` AxisValue)
  (`Controller.SetControlRotation` (`GameplayStatics.GetPlayerController` 0) (`KismetMathLibrary.MakeRotator` 0.0 _returnvalue_pitch _returnvalue_yaw)))

(event `ChangeMesh`
  (params (TargetMesh :type "StaticMeshComponent Object Reference") (NewMesh :type "StaticMesh Object Reference"))
  ;[1 1 1] ChangeMeshCustomEvent
  (`StaticMeshComponent.SetStaticMesh` TargetMesh NewMesh))

(event `InputAxisKey|MouseY`
  (params (AxisValue :type "Float (single-precision)"))
  ;[1 1 1] Camera Controls
  (`self.AddControllerPitchInput` AxisValue))

(event `InputAction|Drift`
  (params (Key :type "Key Structure"))
  (bind _currentfriction (`self.CurrentFriction`))
  ;[1 1 1] Simple Drifting
  (:`Pressed`
    (bind _aschaos_wheeled_vehicle_movement_component (cast `ChaosWheeledVehicleMovementComponent` (`self.VehicleMovementComponent`) :!label _label))
    (`ChaosWheeledVehicleMovementComponent.SetWheelFrictionMultiplier` _aschaos_wheeled_vehicle_movement_component 2 _currentfriction)
    (`ChaosWheeledVehicleMovementComponent.SetWheelFrictionMultiplier` _aschaos_wheeled_vehicle_movement_component 3 _currentfriction))
  (:`Released`
    (if (`self.bIsDrifting`) :!label _label_2
      (goto _label)
      (else
        (bind _aschaos_wheeled_vehicle_movement_component_2 (cast `ChaosWheeledVehicleMovementComponent` (`self.VehicleMovementComponent`)))
        (`ChaosWheeledVehicleMovementComponent.SetWheelFrictionMultiplier` _aschaos_wheeled_vehicle_movement_component_2 2 _currentfriction)
        (`ChaosWheeledVehicleMovementComponent.SetWheelFrictionMultiplier` _aschaos_wheeled_vehicle_movement_component_2 3 _currentfriction)))))

(event `self.ReceiveTick`
  (params (DeltaSeconds :type "Float (single-precision)"))
  ;[1 1 1] Simple Drifting
  (goto _label_2))

(event `InputAction|Reset`
  (params (Key :type "Key Structure"))
  ;[1 1 1] ResetCar
  (:`Pressed`
    (bind _returnvalue (`GameplayStatics.GetCurrentLevelName` true))
    (if (or (`KismetStringLibrary.EqualEqual_StrStr` _returnvalue "Map1") (`KismetStringLibrary.EqualEqual_StrStr` _returnvalue "Map2"))
      (if (not (`self.ResetBool`))
        (set `self.ResetBool` true)
        (`self.ResetCar`)
        (`KismetSystemLibrary.Delay` 5.0)
        (set `self.ResetBool` false)))))

(event `InputAction|Restart`
  (params (Key :type "Key Structure"))
  ;[1 1 1] Restart
  (:`Pressed`
    (bind _returnvalue (`GameplayStatics.GetCurrentLevelName` true))
    (if (or (`KismetStringLibrary.EqualEqual_StrStr` _returnvalue "Map1") (`KismetStringLibrary.EqualEqual_StrStr` _returnvalue "Map2"))
      (bind _outactors (`GameplayStatics.GetAllActorsOfClass` "/Game/Blueprints/BP_StartPoint.BP_StartPoint_C"))
      (for _array_element _outactors
        _)
      (`self.K2_TeleportTo` (`self.K2_GetActorLocation` _array_element) (`self.K2_GetActorRotation` _array_element))
      (`PrimitiveComponent.SetPhysicsLinearVelocity` (`self.Mesh`) (0.0 0.0 0.0) false "None"))))

(event `InputAction|Lights`
  (params (Key :type "Key Structure"))
  ;[1 1 1] Lights
  (:`Pressed`
    (if (`self.LightsOn`)
      (`SceneComponent.SetVisibility` (`self.Headlight`) false false)
      (`SceneComponent.SetVisibility` (`self.Headlight1`) false false)
      (set `self.LightsOn` false)
      (else
        (`SceneComponent.SetVisibility` (`self.Headlight`) true false)
        (`SceneComponent.SetVisibility` (`self.Headlight1`) true false)
        (set `self.LightsOn` true)))))

(fn `UserConstructionScript`)